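; Flashlight component that switches the player's light on and off and manages its battery charge.
; Initialize caches the player's light, and toggling it on starts a looping timer that drains the battery until it empties or is switched off.
; Battery changes are clamped and remapped to the light's IES brightness scale, so the beam dims as charge runs low.
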(fn `AddBatteryLife`
  (params (Amount :type "Float (double-precision)"))
  (set `self.CurrentBatteryLevel` (`KismetMathLibrary.FClamp` (+ (`self.CurrentBatteryLevel`) Amount) (`self.MinBatteryLevel`) (`self.MaxBatteryLevel`)))
  (`self.SetIntensity`))

(fn `DepleteBatteryLife`
  (bind _output_get (set `self.CurrentBatteryLevel` (`KismetMathLibrary.FClamp` (- (`self.CurrentBatteryLevel`) (`self.DepletionAmount`)) (`self.MinBatteryLevel`) (`self.MaxBatteryLevel`))))
  (`self.SetIntensity`)
  (if (<= _output_get (`self.MinBatteryLevel`))
    (`SceneComponent.SetVisibility` (`self.FlashightLight`) false false)
    (`KismetSystemLibrary.K2_ClearTimer` null "DepleteBatteryLife")))

(fn `Initialize`
  (params (Player :type "/Game/gameBP/level1/l1Character Object Reference"))
  (bind _output_get (set `self.PlayerRef` Player))
  (set `self.FlashightLight` (`/Game/gameBP/level1/l1Character.Flashlight` _output_get)))

(fn `SetIntensity`
  (`LightComponent.SetIESBrightnessScale` (`self.FlashightLight`) (`KismetMathLibrary.MapRangeClamped` (`self.CurrentBatteryLevel`) (`self.MinBatteryLevel`) 20.0 0.0 1.0)))

(fn `ToggleFlashlight`
  (bind _flashightlight (`self.FlashightLight`))
  (if (`SceneComponent.bVisible` _flashightlight)
    (`SceneComponent.SetVisibility` _flashightlight false false)
    (`KismetSystemLibrary.K2_ClearTimer` null "DepleteBatteryLife")
    (elif (> (`self.CurrentBatteryLevel`) (`self.MinBatteryLevel`))
      (`self.SetIntensity`)
      (`SceneComponent.SetVisibility` _flashightlight true false)
      (`KismetSystemLibrary.K2_SetTimer` null "DepleteBatteryLife" (`self.DepletionSpeed`) true))))