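; Player inventory component that stores items in a resizable slot array, sized from the player controller, and refreshes the matching grid widget slots on change.
; AddItem fills partial stacks, then empty slots, recursing on overflow and returning any remainder.
; UseItem calls an existing or newly spawned item actor, consuming one on success.
; DropItem spawns the whole stack as a physics pickup at a camera trace, and an examination widget displays chosen items.
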(event `self.ReceiveBeginPlay`
  (`self.Initialize`))

(event `Initialize`
  (bind _assh_player_controller (cast `/Game/gameBP/shPlayerController` (`GameplayStatics.GetPlayerController` 0) :!pure true))
  (`KismetArrayLibrary.Array_Resize` (`self.InventorySlots`) (`/Game/gameBP/shPlayerController.InventorySlots` _assh_player_controller))
  (set `self.WInventoryMenuRef` (`/Game/gameBP/shPlayerController.WInventoryMenuRef` _assh_player_controller))
  (bind _asl_1character (cast `/Game/gameBP/level1/l1Character` (`GameplayStatics.GetPlayerCharacter` 0)))
  (set `self.PlayerRef` _asl_1character)
  (bind _returnvalue (`|CreateWidget` "/Game/UMG/Inventory/WExamination.WExamination_C" null null))
  (set `self.WExaminationRef` _returnvalue)
  (set `/Game/gameBP/shPlayerController.WExaminationRef` (`self.WExaminationRef`) _assh_player_controller)
  (bind _outactors (`GameplayStatics.GetAllActorsOfClass` "/Game/Blueprints/Actors/Inventory/bpExamination.bpExamination_C"))
  (set `self.BpExaminationRef` (`|GetArrayItem` _outactors))
  (set `/Game/UMG/Inventory/WExamination.BpcInventory` self (`self.WExaminationRef`)))

(event `CreateExaminationWidget`
  (params (Index :type Integer))
  (bind _winventorymenuref (`self.WInventoryMenuRef`))
  (`/Game/UMG/Inventory/WExamination.UpdateWidget` (`self.WExaminationRef`) Index)
  (`Widget.SetVisibility` _winventorymenuref "Collapsed")
  (`/Engine/EditorBlueprintResources/StandardMacros.IsValid` (`/Game/UMG/Inventory/WInventoryMenu.WInventoryDropDown` _winventorymenuref)
    (:`Is Valid`
      (`/Game/UMG/Inventory/WInventoryMenu.CloseDropDownMenu` _winventorymenuref))
    (:`Is Not Valid`
      _))
  (`UserWidget.AddToViewport` (`self.WExaminationRef`) 2)
  (set `/Game/gameBP/shPlayerController.IsInventoryOpen` false (cast `/Game/gameBP/shPlayerController` (`GameplayStatics.GetPlayerController` 0) :!pure true)))

(fn `AddItem`
  (params (Item :type "/Game/Blueprints/Actors/Inventory/bpInventoryItemMaster Class Reference") (Amount :type Integer))
  (returns (Success :type Boolean) (Remainder :type Integer))
  (locals (LocalItem :type "/Game/Blueprints/Actors/Inventory/bpInventoryItemMaster Class Reference") (LocalAmount :type Integer) (LocalMaxStackAmount :type Integer) (LocalIndex :type Integer :default 0))
  (bind (_success _index) (`self.CheckForEmptySlot`))
  (bind (_success_2 _index_2) (`self.CheckForEmptySlot`))
  (bind _returnvalue (- (`local.LocalAmount`) 1))
  (bind (_itemname _icon _description _maxstackamount) (break `/Game/Blueprints/Strucs/SItemData` (defaults `Object` (`local.LocalItem`))))
  (bind _returnvalue_2 (+ (`.Amount` (`self.GetItemDataAtIndex` (`local.LocalIndex`))) (`local.LocalAmount`)))
  (set `local.LocalItem` Item)
  (set `local.LocalAmount` Amount)
  (set `local.LocalMaxStackAmount` _maxstackamount)
  (if (> _maxstackamount 1)
    (bind (_success_3 _index_3) (`self.CheckForFreeSlot` (`local.LocalItem`)))
    (if _success_3
      (set `local.LocalIndex` _index_3)
      (if (> _returnvalue_2 (`local.LocalMaxStackAmount`))
        (set `local.LocalAmount` (- _returnvalue_2 (`local.LocalMaxStackAmount`)))
        (`KismetArrayLibrary.Array_Set` (`self.InventorySlots`) (`local.LocalIndex`) (make `/Game/Blueprints/Strucs/SInventoryItems` (`local.LocalItem`) (`local.LocalMaxStackAmount`)))
        (`self.UpdateInventorySlot` (`local.LocalIndex`))
        (bind (_success_4 _remainder) (`self.AddItem` (`local.LocalItem`) (`local.LocalAmount`)))
        (return true _remainder)
        (else
          (`KismetArrayLibrary.Array_Set` (`self.InventorySlots`) (`local.LocalIndex`) (make `/Game/Blueprints/Strucs/SInventoryItems` (`local.LocalItem`) _returnvalue_2))
          (`self.UpdateInventorySlot` (`local.LocalIndex`))
          (return true 0)))
      (elif _success
        (set `local.LocalIndex` _index)
        (if (> (`local.LocalAmount`) (`local.LocalMaxStackAmount`))
          (`KismetArrayLibrary.Array_Set` (`self.InventorySlots`) (`local.LocalIndex`) (make `/Game/Blueprints/Strucs/SInventoryItems` (`local.LocalItem`) (`local.LocalMaxStackAmount`)))
          (`self.UpdateInventorySlot` (`local.LocalIndex`))
          (bind (_success_5 _remainder_2) (`self.AddItem` (`local.LocalItem`) (- (`local.LocalAmount`) (`local.LocalMaxStackAmount`))))
          (return true _remainder_2)
          (else
            (`KismetArrayLibrary.Array_Set` (`self.InventorySlots`) (`local.LocalIndex`) (make `/Game/Blueprints/Strucs/SInventoryItems` (`local.LocalItem`) (`local.LocalAmount`)))
            (`self.UpdateInventorySlot` (`local.LocalIndex`))
            (return true 0)))
        (else
          (return false (`local.LocalAmount`)))))
    (elif _success_2
      (set `local.LocalIndex` _index_2)
      (`KismetArrayLibrary.Array_Set` (`self.InventorySlots`) (`local.LocalIndex`) (make `/Game/Blueprints/Strucs/SInventoryItems` (`local.LocalItem`) 1))
      (`self.UpdateInventorySlot` (`local.LocalIndex`))
      (if (> _returnvalue 0)
        (bind (_success_6 _remainder_3) (`self.AddItem` (`local.LocalItem`) _returnvalue))
        (return true _remainder_3)
        (else
          (return true 0)))
      (else
        (`KismetSystemLibrary.PrintString` "No free slots")
        (return false (`local.LocalAmount`))))))

(fn `AddMoreSlots`
  (params (Amount :type Integer))
  (bind _winventorymenuref (`self.WInventoryMenuRef`))
  (bind _assh_player_controller (cast `/Game/gameBP/shPlayerController` (`GameplayStatics.GetPlayerController` 0) :!pure true))
  (bind _winventorygrid (`/Game/UMG/Inventory/WInventoryMenu.WInventoryGrid` _winventorymenuref))
  (bind _output_get (set `/Game/gameBP/shPlayerController.InventorySlots` (+ Amount (`/Game/gameBP/shPlayerController.InventorySlots` _assh_player_controller)) _assh_player_controller))
  (`KismetArrayLibrary.Array_Resize` (`self.InventorySlots`) _output_get)
  (`/Game/UMG/Inventory/WInventoryGrid.AddMoreSlots` _winventorygrid Amount)
  (for _array_element (`/Game/UMG/Inventory/WInventoryGrid.SlotsArray` _winventorygrid)
    (`/Game/UMG/Inventory/WInventorySlot.Initialize` _array_element _winventorymenuref)))

(fn `CheckForEmptySlot`
  (returns (Success :type Boolean) (Index :type Integer))
  (locals (LocalSuccess :type Boolean) (LocalIndex :type Integer))
  (for (_array_element _array_index) (`self.InventorySlots`)
    (if (`KismetSystemLibrary.IsValidClass` (`.Item_4_01776BFF4523179748C7C09872FD74F7` (break `/Game/Blueprints/Strucs/SInventoryItems` _array_element)))
      (set `local.LocalSuccess` false)
      (else
        (set `local.LocalSuccess` true)
        (set `local.LocalIndex` _array_index)
        (break))))
  (return (`local.LocalSuccess`) (`local.LocalIndex`)))

(fn `CheckForFreeSlot`
  (params (Item :type "/Game/Blueprints/Actors/Inventory/bpInventoryItemMaster Class Reference"))
  (returns (Success :type Boolean) (Index :type Integer))
  (locals (LocalSuccess :type Boolean) (localIndex :type Integer))
  (for (_array_element _array_index) (`self.InventorySlots`)
    (bind (_item _amount) (break `/Game/Blueprints/Strucs/SInventoryItems` _array_element))
    (if (and (== _item Item) (< _amount (`.MaxStackAmount_9_E4155346441D09ECDF116D957EED6F64` (break `/Game/Blueprints/Strucs/SItemData` (defaults `Object` Item)))))
      (set `local.LocalSuccess` true)
      (set `local.localIndex` _array_index)
      (break)
      (else
        (set `local.LocalSuccess` false))))
  (return (`local.LocalSuccess`) (`local.localIndex`)))

(fn `DropItem`
  (params (Index :type Integer))
  (locals (LocalIndex :type Integer) (LocalAmount :type Integer :default 0) (LocalItem :type "/Game/Blueprints/Actors/Inventory/bpInventoryItemMaster Class Reference"))
  (bind _camera (`/Game/gameBP/level1/l1Character.Camera` (`self.PlayerRef`)))
  (bind _returnvalue (`SceneComponent.K2_GetComponentLocation` _camera))
  (bind _output_get (set `local.LocalIndex` Index))
  (bind (_item _amount) (`self.GetItemDataAtIndex` _output_get))
  (set `local.LocalAmount` _amount)
  (set `local.LocalItem` _item)
  (if (> (`local.LocalAmount`) 0)
    (for _ (range (`local.LocalAmount`))
      (`self.RemoveItem` (`local.LocalIndex`)))
    (`/Game/UMG/Inventory/WInventoryMenu.CloseDropDownMenu` (`self.WInventoryMenuRef`))
    (bind (_outhit _returnvalue_2) (`KismetSystemLibrary.LineTraceSingle` _returnvalue (+ _returnvalue (* (`SceneComponent.GetForwardVector` _camera) 200.0)) "TraceTypeQuery1"))
    (bind (_bblockinghit _binitialoverlap _time _distance _location _impactpoint _normal _impactnormal _physmat _hitactor _hitcomponent _hitbonename _bonename _hititem _elementindex _faceindex _tracestart _traceend) (`GameplayStatics.BreakHitResult` _outhit))
    (bind _returnvalue_3 (`|SpawnActorFromClass` (`.PickUpActor_16_E9494DC044A8A1D154F1A183E62754E6` (break `/Game/Blueprints/Strucs/SItemData` (defaults `Object` (`local.LocalItem`)))) (`KismetMathLibrary.MakeTransform` (select `bool` _returnvalue_2 :`false` _traceend :`true` _location)) "Undefined" "OverrideRootScale" null null))
    (set `/Game/Blueprints/Actors/Inventory/PickUpActors/bpPickUpActorMaster.Amount` (`local.LocalAmount`) _returnvalue_3)
    (`PrimitiveComponent.SetSimulatePhysics` (`/Game/Blueprints/Actors/Inventory/PickUpActors/bpPickUpActorMaster.StaticMesh` _returnvalue_3) true)))

(fn `GetItemDataAtIndex`
  (params (Index :type Integer))
  (returns (Item :type "/Game/Blueprints/Actors/Inventory/bpInventoryItemMaster Class Reference") (Amount :type Integer))
  (bind (_item _amount) (break `/Game/Blueprints/Strucs/SInventoryItems` (`|GetArrayItem` (`self.InventorySlots`) Index)))
  (return _item _amount))

(fn `RemoveItem`
  (params (Index :type Integer))
  (bind (_item _amount) (`self.GetItemDataAtIndex` Index))
  (if (> _amount 1)
    (`KismetArrayLibrary.Array_Set` (`self.InventorySlots`) Index (make `/Game/Blueprints/Strucs/SInventoryItems` _item (- _amount 1)))
    (else
      (`KismetArrayLibrary.Array_Set` (`self.InventorySlots`) Index (make `/Game/Blueprints/Strucs/SInventoryItems` null))))
  (`self.UpdateInventorySlot` Index))

(fn `UpdateInventorySlot`
  (params (Index :type Integer))
  (`/Game/UMG/Inventory/WInventorySlot.UpdateSlot` (`|GetArrayItem` (`/Game/UMG/Inventory/WInventoryGrid.SlotsArray` (`/Game/UMG/Inventory/WInventoryMenu.WInventoryGrid` (`/Game/gameBP/shPlayerController.WInventoryMenuRef` (cast `/Game/gameBP/shPlayerController` (`GameplayStatics.GetPlayerController` 0) :!pure true)))) Index)))

(fn `UseItem`
  (params (Index :type Integer))
  (locals (LocalIndex :type Integer))
  (bind _output_get (set `local.LocalIndex` Index))
  (bind (_item _amount) (`self.GetItemDataAtIndex` _output_get))
  (if (> _amount 0)
    (bind _returnvalue (`GameplayStatics.GetActorOfClass` _item))
    (`/Engine/EditorBlueprintResources/StandardMacros.IsValid` null
      (:`Is Valid`
        (`/Game/Blueprints/Actors/Inventory/bpInventoryItemMaster.UseItem` _returnvalue)
        (if (`/Game/Blueprints/Actors/Inventory/bpInventoryItemMaster.UseItemSuccess` _returnvalue)
          (`self.RemoveItem` (`local.LocalIndex`) :!label _label)
          (`/Game/UMG/Inventory/WInventoryMenu.CloseDropDownMenu` (`self.WInventoryMenuRef`))
          (else
            (`KismetSystemLibrary.PrintString` "Use Item Not Successful" :!label _label_2))))
      (:`Is Not Valid`
        (bind _returnvalue_2 (`|SpawnActorFromClass` _item (`KismetMathLibrary.MakeTransform` (0.0 0.0 0.0)) "Undefined" "OverrideRootScale" null null))
        (`/Game/Blueprints/Actors/Inventory/bpInventoryItemMaster.UseItem` _returnvalue_2)
        (if (`/Game/Blueprints/Actors/Inventory/bpInventoryItemMaster.UseItemSuccess` _returnvalue_2)
          (goto _label)
          (else
            (goto _label_2)))))))